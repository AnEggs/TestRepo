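; Player hero character for a twin-stick shooter, with stick movement, aim-to-fire shooting and a screen-clearing nuke.
; BeginPlay attaches a weapon to the gun socket, stores the spawn point in TwinStickMode and creates the HUD and nuke button.
; Look input past a deadzone rotates and fires; Nuke, from input or the button rebound every Tick, zeroes all enemies' health.
; Death disables input and shows a delayed death screen; RespawnHero resets score, respawns and destroys hero and weapon.
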(event `self.ReceiveBeginPlay`
  (bind _mesh (`self.Mesh`))
  (`|ExecutionSequence`
    (:`then_0`
      (bind _returnvalue (`|SpawnActorFromClass` "/Game/BluePrints/Weapon.Weapon_C" (`SceneComponent.K2_GetComponentToWorld` _mesh) "Undefined" "OverrideRootScale" null null))
      (bind _output_get (set `self.Weapon` _returnvalue))
      (`self.K2_AttachRootComponentTo` _output_get _mesh "GunSocket" "SnapToTarget" true))
    (:`then_1`
      (bind _astwin_stick_mode (cast `/Game/BluePrints/TwinStickMode` (`GameplayStatics.GetGameMode`)))
      (bind _output_get_2 (set `self.GameMode` _astwin_stick_mode))
      (set `/Game/BluePrints/TwinStickMode.PlayerSpawnLocation` (`self.GetTransform`) _output_get_2))
    (:`then_2`
      (bind _returnvalue_2 (`|CreateWidget` "/Game/BluePrints/TwinStickHUD.TwinStickHUD_C"))
      (`UserWidget.AddToViewport` _returnvalue_2 0))
    (:`then_3`
      (bind _returnvalue_3 (`|CreateWidget` "/Game/NukeButton.NukeButton_C"))
      (`UserWidget.AddToViewport` _returnvalue_3 0))))

(event `self.ReceiveTick`
  (params (DeltaSeconds :type "Float (single-precision)"))
  (add `/Game/NukeButton.NukeDispatcher` (stale `self.ReceiveBeginPlay` _returnvalue_3) (delegate `Nuke`)))

(event `InputAxis|MoveUp`
  (params (AxisValue :type "Float (single-precision)"))
  ;[1 1 1] Movement
  (`self.AddMovementInput` (1.0 0.0 0.0) AxisValue))

(event `InputAxis|LookUp`
  (params (AxisValue :type "Float (single-precision)"))
  (bind _weapon (`self.Weapon`))
  ;[1 1 1] Rotation
  (bind _returnvalue (`KismetMathLibrary.MakeVector` AxisValue (stale `InputAxis|LookRight` AxisValue)))
  (if (> (`KismetMathLibrary.VSize` _returnvalue) 0.25) :!label _label
    (`Controller.SetControlRotation` (`self.GetController`) (`KismetMathLibrary.Conv_VectorToRotator` _returnvalue))
    ;[1 1 1] Shoot
    (`/Game/BluePrints/Weapon.PullTrigger` _weapon)
    (else
      (`/Game/BluePrints/Weapon.ReleaseTrigger` _weapon))))

(event `InputAxis|MoveRight`
  (params (AxisValue :type "Float (single-precision)"))
  ;[1 1 1] Movement
  (`self.AddMovementInput` (0.0 1.0 0.0) AxisValue))

(event `InputAxis|LookRight`
  (params (AxisValue :type "Float (single-precision)"))
  ;[1 1 1] Rotation
  (goto _label))

(event `InputAction|Nuke`
  (params (Key :type "Key Structure"))
  (:`Pressed`
    (`self.Nuke` self)))

(event `Nuke`
  (`|ExecutionSequence`
    (:`then_0`
      (bind _outactors (`GameplayStatics.GetAllActorsOfClass` "/Game/BluePrints/EnemyCharacter.EnemyCharacter_C"))
      (for _array_element _outactors
        (set `/Game/BaseCharacter.Health` 0.0 _array_element)
        (bind _asenemy_character (cast `/Game/BluePrints/EnemyCharacter` _array_element))
        (`self.AffectHealth` _asenemy_character 0.0)))))

(event `self.AffectHealth`
  (params (Delta :type "Float (single-precision)"))
  (`self.CalcHealth` Delta)
  (`KismetSystemLibrary.PrintString` (`KismetStringLibrary.Conv_DoubleToString` (`self.Health`)))
  (if (`self.IsDead`)
    (`self.DisableInput` null)
    (`KismetSystemLibrary.Delay` 3.0)
    (bind _returnvalue (`|CreateWidget` "/Game/DeathScreen.DeathScreen_C" (`GameplayStatics.GetPlayerController` 0)))
    (`UserWidget.AddToViewport` _returnvalue 0)))

(fn `RespawnHero`
  (bind _gamemode (`self.GameMode`))
  (`/Game/BluePrints/TwinStickMode.ResetScore` _gamemode)
  (`/Game/BluePrints/TwinStickMode.RespawnPlayer` _gamemode)
  (`self.K2_DestroyActor` (`self.Weapon`))
  (`self.K2_DestroyActor` self))

(fn `UserConstructionScript`
  (`parent.UserConstructionScript`))
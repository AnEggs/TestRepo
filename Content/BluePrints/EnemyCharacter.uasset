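; Enemy character for a twin-stick game that bites the hero on overlap and dies when its health runs out.
; Overlapping the hero starts a looping attack timer that deals damage until overlap ends or the hero dies.
; Death ragdolls the mesh, credits score and nuke progress to TwinStickMode, then spawns a delayed explosion before destroying the actor.
; The construction script creates a dynamic material and sets its body colour.
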(event `self.ReceiveBeginPlay`)

(event `/Game/BluePrints/iDamageable.AffectHealth`
  (params (Delta :type "Float (single-precision)"))
  (bind _capsulecomponent (`self.CapsuleComponent`))
  (`self.CalcHealth` Delta)
  (if (`self.IsDead`)
    (`ActorComponent.K2_DestroyComponent` (`self.DamageVolume`))
    (`PrimitiveComponent.SetSimulatePhysics` (`self.Mesh`) true)
    (`PrimitiveComponent.SetCollisionResponseToChannel` _capsulecomponent "ECC_WorldDynamic" "ECR_Ignore")
    (`PrimitiveComponent.SetCollisionResponseToChannel` _capsulecomponent "ECC_Pawn" "ECR_Ignore")
    (`KismetSystemLibrary.PrintString` "Enemy Killed")
    (bind _astwin_stick_mode (cast `/Game/BluePrints/TwinStickMode` (`GameplayStatics.GetGameMode`)))
    (`/Game/BluePrints/TwinStickMode.IncrementScore` _astwin_stick_mode (`self.Score`))
    (`/Game/BluePrints/TwinStickMode.IncrementNuke` _astwin_stick_mode (`self.NukeKills`))
    (`self.DetachFromControllerPendingDestroy`)
    (`KismetSystemLibrary.Delay` 2.0)
    (`|SpawnActorFromClass` "/Game/BluePrints/Explosion.Explosion_C" (`self.GetTransform`) "Undefined" "OverrideRootScale" null null)
    (`KismetSystemLibrary.Delay` 3.0)
    (`self.K2_DestroyActor`)))

(event `self.ReceiveActorBeginOverlap`
  (params (OtherActor :type "Actor Object Reference"))
  (bind _ashero_character (cast `/Game/BluePrints/HeroCharacter` OtherActor))
  (set `self.Hero` _ashero_character)
  (set `CharacterMovementComponent.MaxWalkSpeed` 0.0 (`self.CharacterMovement`))
  (set `self.IsBiting` true)
  (`KismetSystemLibrary.K2_SetTimer` null "DamageTheHero" (/ 1.0 (`self.AttacksPerSecond`)) true)
  (set `CharacterMovementComponent.MaxWalkSpeed` 200.0 (`self.CharacterMovement`)))

(event `DamageTheHero`
  (if (not (`self.IsDead`))
    (`/Game/BluePrints/HeroCharacter.AffectHealth` (`self.Hero`) (`self.Damage`))
    (bind _ashero_character (cast `/Game/BluePrints/HeroCharacter` (stale `self.ReceiveActorBeginOverlap` OtherActor)))
    (if (`/Game/BaseCharacter.IsDead` _ashero_character)
      (`KismetSystemLibrary.K2_ClearTimer` null "DamageTheHero"))))

(event `self.ReceiveActorEndOverlap`
  (params (OtherActor :type "Actor Object Reference"))
  (if (== OtherActor (`self.Hero`))
    (`KismetSystemLibrary.K2_ClearTimer` null "DamageTheHero")
    (set `self.IsBiting` false)))

(fn `UserConstructionScript`
  (`parent.UserConstructionScript`)
  (bind _returnvalue (`PrimitiveComponent.CreateDynamicMaterialInstance` (`self.Mesh`) 0 null))
  (bind _output_get (set `self.DynoMat` _returnvalue))
  (`MaterialInstanceDynamic.SetVectorParameterValue` :`self` _output_get :`ParameterName` "BodyColor"))
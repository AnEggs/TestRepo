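; Projectile is a laser shot actor that damages hostile actors on contact.
; On overlap, it sends its Damage value through the IDamageable interface to any implementer not tagged Friendly.
; Every overlap, including with friendly or non-damageable actors, then triggers a laser hit sound attached to its sphere collision, spawns GPU spark particles at its location and destroys the projectile.
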(event `self.ReceiveActorBeginOverlap`
  (params (OtherActor :type "Actor Object Reference"))
  (bind (_returnvalue_location _returnvalue_rotation) (`KismetMathLibrary.BreakTransform` (`self.GetTransform`)))
  (if (`KismetSystemLibrary.DoesImplementInterface` OtherActor "/Game/BluePrints/iDamageable.iDamageable_C")
    (if (not (`self.ActorHasTag` OtherActor "Friendly"))
      (message `/Game/BluePrints/iDamageable.AffectHealth` OtherActor (`self.Damage`))))
  (`GameplayStatics.SpawnSoundAttached` "/Game/Audio/LaserHit.LaserHit" (`self.SphereCollision`))
  (`GameplayStatics.SpawnEmitterAtLocation` "/Game/StarterContent/Particles/P_LaserSparksGPU.P_LaserSparksGPU" _returnvalue_location _returnvalue_rotation)
  (`self.K2_DestroyActor`))

(fn `UserConstructionScript`)